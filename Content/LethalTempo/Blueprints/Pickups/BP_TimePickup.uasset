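; BP_TimePickup is a respawning pickup that adds seconds to the HorrorEngineCharacter timer when the player overlaps its Trigger.
; Collection also plays a 2D sound and calls HealthIconCheck on the HealthWB widget.
; It then hides itself, spawns BP_CooldownText at NSPickup3, and after a fixed delay removes the text and reappears.
; An OnCooldown flag blocks collection while hidden.
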(event `self.Trigger.OnComponentBeginOverlap`
  (params (OverlappedComponent :type "PrimitiveComponent Object Reference") (OtherActor :type "Actor Object Reference") (OtherComp :type "PrimitiveComponent Object Reference") (OtherBodyIndex :type Integer) (bFromSweep :type Boolean) (SweepResult :type "HitResult Structure (by ref)"))
  (if (== (`self.OnCooldown`) false)
    (if (== OtherActor (`GameplayStatics.GetPlayerPawn` 0))
      (`|ExecutionSequence`
        (:`then_0`
          (bind _ashorror_engine_character (cast `/Game/HorrorEngine/Blueprints/Core/HorrorEngineCharacter` (`GameplayStatics.GetPlayerPawn` 0)))
          (set `/Game/HorrorEngine/Blueprints/Core/HorrorEngineCharacter.TimerSeconds` (+ (`/Game/HorrorEngine/Blueprints/Core/HorrorEngineCharacter.TimerSeconds` _ashorror_engine_character) 10) _ashorror_engine_character))
        (:`then_1`
          (`/Game/HorrorEngine/Blueprints/Core/HorrorEngineFunctions.GetPlayer`)
          (`/Game/HorrorEngine/Blueprints/Core/HorrorEngineMacros.HM_2DSound` null true)
          (bind _foundwidgets (`WidgetBlueprintLibrary.GetAllWidgetsOfClass` "/Game/HorrorEngine/Blueprints/Widgets/SubWidgets/HealthWB.HealthWB_C" false))
          (`/Game/HorrorEngine/Blueprints/Widgets/SubWidgets/HealthWB.HealthIconCheck` _foundwidgets)
          (set `self.OnCooldown` true)
          (`self.SetActorHiddenInGame` true)
          (bind _returnvalue (`|SpawnActorFromClass` "/Game/LethalTempo/Blueprints/Pickups/BP_CooldownText.BP_CooldownText_C" (`SceneComponent.K2_GetComponentToWorld` (`self.NS_Pickup_3`)) "AlwaysSpawn" "MultiplyWithRoot" null null))
          (`KismetSystemLibrary.Delay` 15.0)
          (`self.K2_DestroyActor` _returnvalue)
          (`self.SetActorHiddenInGame` false)
          (set `self.OnCooldown` false))))))

(fn `UserConstructionScript`)