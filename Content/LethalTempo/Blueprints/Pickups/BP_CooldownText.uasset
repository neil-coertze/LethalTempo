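; BP_CooldownText is a pickup-related Blueprint that displays a countdown of the remaining cooldown as text.
; BeginPlay writes the initial CurrentCooldown to CooldownTime.
; Tick runs into a one-second Delay, which ignores re-triggers while pending, so the value drops by one and the text refreshes roughly every second.
; The file shows no stop at zero.
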(event `self.ReceiveBeginPlay`
  (`TextRenderComponent.K2_SetText` (`self.CooldownTime`) (`KismetTextLibrary.Conv_IntToText` (`self.CurrentCooldown`))))

(event `self.ReceiveTick`
  (params (DeltaSeconds :type "Float (single-precision)"))
  (`KismetSystemLibrary.Delay` 1.0)
  (bind _output_get (set `self.CurrentCooldown` (- (`self.CurrentCooldown`) 1)))
  (`TextRenderComponent.K2_SetText` (`self.CooldownTime`) (`KismetTextLibrary.Conv_IntToText` _output_get)))

(fn `UserConstructionScript`)