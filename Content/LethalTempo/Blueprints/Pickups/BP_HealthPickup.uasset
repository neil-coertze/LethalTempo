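; Health pickup that grants the player a fixed amount of health on overlap, then goes on a timed cooldown and respawns.
; At full health it only shows a notice; otherwise it plays a sound and refreshes the HealthWB widget's icon.
; During cooldown a flag blocks reuse while the actor is hidden and a spawned BP_CooldownText stands in until the delay ends.
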(event `self.Trigger.OnComponentBeginOverlap`
  (params (OverlappedComponent :type "PrimitiveComponent Object Reference") (OtherActor :type "Actor Object Reference") (OtherComp :type "PrimitiveComponent Object Reference") (OtherBodyIndex :type Integer) (bFromSweep :type Boolean) (SweepResult :type "HitResult Structure (by ref)"))
  (if (== (`self.OnCooldown`) false)
    (if (== OtherActor (`GameplayStatics.GetPlayerPawn` 0))
      (bind _asmaster (`/Game/HorrorEngine/Blueprints/Core/HorrorEngineFunctions.GetPlayer`))
      (if (== (`/Game/HorrorEngine/HorrorEngine.Health` _asmaster) 100.0)
        (`/Game/HorrorEngine/Blueprints/Core/HorrorEngineFunctions.Notice` "" "Health" "is full!")
        (else
          (`/Game/HorrorEngine/HorrorEngine.GetHealth` _asmaster 20.0)
          (`/Game/HorrorEngine/Blueprints/Core/HorrorEngineMacros.HM_2DSound` null true)
          (bind _foundwidgets (`WidgetBlueprintLibrary.GetAllWidgetsOfClass` "/Game/HorrorEngine/Blueprints/Widgets/SubWidgets/HealthWB.HealthWB_C" false))
          (`/Game/HorrorEngine/Blueprints/Widgets/SubWidgets/HealthWB.HealthIconCheck` _foundwidgets)
          (set `self.OnCooldown` true)
          (`self.SetActorHiddenInGame` true)
          (bind _returnvalue (`|SpawnActorFromClass` "/Game/LethalTempo/Blueprints/Pickups/BP_CooldownText.BP_CooldownText_C" (`SceneComponent.K2_GetComponentToWorld` (`self.NS_Pickup_3`)) "Undefined" "MultiplyWithRoot" null null))
          (`KismetSystemLibrary.Delay` 15.0)
          (`self.K2_DestroyActor` _returnvalue)
          (`self.SetActorHiddenInGame` false)
          (set `self.OnCooldown` false))))))

(fn `UserConstructionScript`)